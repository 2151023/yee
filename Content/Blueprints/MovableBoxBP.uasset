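; Movable box actor that tells the BoxesPlayerController when the player character enters or leaves its overlap area.
; Begin and end overlap events pass the box itself to the controller's trigger enter and leave dispatcher calls.
; GetTargetPlayerTransform supplies a player target from the Trigger's position and rotation, keeping the player's own height when that actor is valid.
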(event Collision|EventActorBeginOverlap
  (params (OtherActor :type Actor%20Object%20Reference))
  ;[1 1 1] Notify player controller of collision events
  (if (== OtherActor (Game|GetPlayerCharacter 0))
    (bind _asboxes_player_controller (Utilities|Casting|CastToBoxesPlayerController (Game|GetPlayerController 0)))
    (Default|CallBoxTriggerEnterDispatcher _asboxes_player_controller self)))

(event Collision|EventActorEndOverlap
  (params (OtherActor :type Actor%20Object%20Reference))
  ;[1 1 1] Notify player controller of collision events
  (if (== OtherActor (Game|GetPlayerCharacter 0))
    (bind _asboxes_player_controller (Utilities|Casting|CastToBoxesPlayerController (Game|GetPlayerController 0)))
    (Default|CallBoxTriggerLeaveDispatcher _asboxes_player_controller self)))

(fn ConstructionScript)

(fn GetTargetPlayerTransform
  (params (PlayerActor :type Actor%20Object%20Reference))
  (bind _trigger (Variables|Default|GetTrigger))
  (bind _returnvalue (Transformation|GetWorldLocation _trigger))
  (return (Math|Transform|MakeTransform (Math|Vector|MakeVector (.x _returnvalue) (.y _returnvalue) (Math|Float|SelectFloat (.z (Transformation|GetActorLocation PlayerActor)) (.z _returnvalue) (Utilities|IsValid PlayerActor))) (Transformation|GetWorldRotation (Variables|Default|GetTrigger)) "1,1,1")))