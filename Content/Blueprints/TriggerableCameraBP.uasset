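; TriggerableCameraBP is a camera actor that takes over the first player controller's view when a GaltrilianCharacter enters its referenced trigger.
; The construction script binds the trigger's overlap events and draws a debug arrow to trigger boxes.
; Overlaps blend the view in and optionally back out, while Tick can smoothly rotate the camera toward the stored player.
; BoxesGameState class defaults toggle both the return and the tracking.
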(event Custom|OnActorLeaveTrigger
  (params (TriggerActor :type Actor%20Object%20Reference) (PlayerActor :type Actor%20Object%20Reference))
  ;[1 1 1] Reset the camera to the player
  (if (.ReturnToPlayerCameraOnLeaveTrigger (Utilities|GetClassDefaults "/Game/Blueprints/BoxesGameState.BoxesGameState_C"))
    (Variables|Default|SetPlayer 0) ; Unset player
    (Game|Player|SetViewTargetwithBlend (Game|GetPlayerController 0) PlayerActor 1.0 "VTBlend_EaseInOut" 2.0 true)))

(event Custom|OnActorEnterTrigger
  (params (TriggerActor :type Actor%20Object%20Reference) (PlayerActor :type Actor%20Object%20Reference))
  ;[1 1 1] Switch to this camera when a player touches the trigger
  (bind _asgaltrilian_character (Utilities|Casting|CastToGaltrilianCharacter PlayerActor))
  (Utilities|FlowControl|Sequence
    (:then_0
      (Utilities|IsValid (Variables|Default|GetPlayer)
        (:Is%20Not%20Valid
          (Variables|Default|SetPlayer _asgaltrilian_character))))
    (:then_1
      (Game|Player|SetViewTargetwithBlend (Game|GetPlayerController 0) self 1.0 "VTBlend_EaseInOut" 2.0 true))))

(event EventTick
  (params (DeltaSeconds :type Float%20%28single-precision%29))
  (bind _camera (Variables|Default|GetCamera))
  (bind _player (Variables|Default|GetPlayer))
  ;[1 1 1] Look at player
  (if (.TrackPlayerEveryFrame (Utilities|GetClassDefaults "/Game/Blueprints/BoxesGameState.BoxesGameState_C"))
    (Utilities|IsValid _player
      (:Is%20Valid
        (Transformation|SetWorldRotation _camera (Math|Interpolation|RInterpTo (Transformation|GetWorldRotation _camera) (Math|Rotator|FindLookatRotation (Transformation|GetWorldLocation _camera) (Transformation|GetActorLocation _player)) (Utilities|Time|GetWorldDeltaSeconds) 1e+01) false false)))))

(fn ConstructionScript
  (Utilities|IsValid (Variables|Default|GetTriggerReference)
    (:Is%20Valid
      (Utilities|FlowControl|Sequence
        (:then_0
          ;[1 1 1] Draw an arrow to the referenced trigger
          (bind _astrigger_box (Utilities|Casting|CastToTriggerBox (Variables|Default|GetTriggerReference)))
          (Rendering|Debug|DrawDebugArrow (Transformation|GetWorldLocation (Variables|Default|GetCamera)) (Transformation|GetActorLocation _astrigger_box) 1e+03 "(R=0.008736,G=0.000000,B=1.000000,A=1.000000)" 5.0 8.0))
        (:then_1
          ;[1 1 1] Bind trigger's collision event
          (Collision|BindEventtoOnActorBeginOverlap (Variables|Default|GetTriggerReference) (EventDispatchers|CreateEvent :!event Custom|OnActorEnterTrigger))
          (Collision|BindEventtoOnActorEndOverlap (Variables|Default|GetTriggerReference) (EventDispatchers|CreateEvent :!event Custom|OnActorLeaveTrigger)))))))